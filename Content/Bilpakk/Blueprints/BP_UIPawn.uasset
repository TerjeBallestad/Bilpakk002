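; UI pawn that runs the level-select, pause and game-over menus through three widget components.
; Level list fills from a data table; selection updates the game state, map grid and preview container.
; Action bar drives play, continue, menu and quit; play fades out, then calls GameState.StartGame or opens Main with a RowName option.
; Pause shows the picker first, highscores thereafter; Finish shows a popover with drumroll and timeline-animated score.
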(event Custom|ContinueButtonClicked
  (bind _endgamewidget (Variables|Default|GetEndGameWidget))
  (bind _actionbarwidget (Variables|Default|GetActionBarWidget))
  ;[1 1 1] Continue button clicked (Game finished)
  (Widget|SetVisibility _endgamewidget "Collapsed")
  (Widget|SetIsEnabled _endgamewidget false)
  (Widget|SetIsEnabled (Variables|Default|GetPauseAndEndWidget) true)
  (Widget|SetIsEnabled (Variables|Default|GetActionBarWidget) true)
  (Default|EnableMenu _actionbarwidget)
  (Default|EnableMenu _actionbarwidget))

(event Custom|OnPressedPlay
  ;[1 1 1] New Game Pressed
  (|AnimateAndStartNewGame))

(event Custom|OnRowChanged
  (params (Item :type Object%20Object%20Reference) (bIsSelected :type Boolean))
  (bind _gamestate (Variables|Default|GetGameState))
  ;[1 1 1] Selected Different Level In the list
  (bind _asulevel_name_data (Utilities|Casting|CastToULevelNameData Item))
  (bind _output_get (Variables|Default|SetCurrentRow (Variables|/Game/Bilpakk/Data/ULevelNameData.ULevelNameData_C|GetRowName _asulevel_name_data)))
  (bind _returnvalue (Utilities|GetDataTableRow (Variables|Default|GetLevelDataTable) _output_get)
    (:then
      (Utilities|IsValid _gamestate
        (:Is%20Valid
          (Variables|/Script/Bilpakk002.BilpakkGameState|SetLevelData _gamestate _returnvalue))
        (:Is%20Not%20Valid
          _))
      (Default|OnRowChanged (Variables|/Game/Bilpakk/UI/Widgets/WBP_PauseAndEnd.WBP_PauseAndEnd_C|GetWBP_MapGrid (Variables|Default|GetPauseAndEndWidget)) _returnvalue)
      (bind _asbp_preview_container (Utilities|Casting|CastToBP_PreviewContainer (Variables|/Script/Engine.ChildActorComponent|GetChildActor (Variables|Default|GetBP_PreviewContainer))))
      (Default|SetupLevelData _asbp_preview_container _returnvalue))))

(event Custom|ContinuePressed
  (bind _gamestate (Variables|Default|GetGameState))
  ;[1 1 1] Continue
  (if (Variables|/Script/Bilpakk002.BilpakkGameState|GetIsFinished _gamestate)
    (Default|ShowLevelPicker (Variables|Default|GetPauseAndEndWidget))
    (Default|DisableContinue (Variables|Default|GetActionBarWidget))
    (else
      (Class|BilpakkGameState|TogglePause _gamestate))))

(event Custom|MenuPressed
  (bind _actionbarwidget (Variables|Default|GetActionBarWidget))
  ;[1 1 1] Open Level picker
  (Default|ShowLevelPicker (Variables|Default|GetPauseAndEndWidget))
  (Default|DisableMenu _actionbarwidget)
  (Default|EnableNewGame _actionbarwidget))

(event Custom|QuitPressed
  ;[1 1 1] Quit game
  (Game|QuitGame 0 "Quit" false))

(event EventBeginPlay
  (bind _leveldatatable (Variables|Default|GetLevelDataTable))
  (Utilities|FlowControl|Sequence
    (:then_0
      ;[1 1 1] Main widget setup
      (bind _aswbp_pause_and_end (Utilities|Casting|CastToWBP_PauseAndEnd (UserInterface|GetUserWidgetObject (Variables|Default|GetMainUI))))
      (Variables|Default|SetPauseAndEndWidget _aswbp_pause_and_end))
    (:then_1
      ;[1 1 1] Setup level selection list
      (bind _outrownames (DataTable|GetDataTableRowNames _leveldatatable))
      (for _array_element _outrownames
        (bind _returnvalue (Utilities|GetDataTableRow _leveldatatable _array_element)
          (:then
            (Default|AddDatatoList (Variables|/Game/Bilpakk/UI/Widgets/WBP_MapGrid.WBP_MapGrid_C|GetWBP_LevelScroll (Variables|/Game/Bilpakk/UI/Widgets/WBP_PauseAndEnd.WBP_PauseAndEnd_C|GetWBP_MapGrid (Variables|Default|GetPauseAndEndWidget))) _array_element _returnvalue)
            (Default|Setup (Variables|/Game/Bilpakk/UI/Widgets/WBP_PauseAndEnd.WBP_PauseAndEnd_C|GetWBP_MapGrid (Variables|Default|GetPauseAndEndWidget)) _returnvalue)
            (EventDispatchers|BindEventtoBPonItemSelectionChanged (Variables|/Game/Bilpakk/UI/Widgets/WBP_LevelScroll.WBP_LevelScroll_C|GetLevels (Variables|/Game/Bilpakk/UI/Widgets/WBP_MapGrid.WBP_MapGrid_C|GetWBP_LevelScroll (Variables|/Game/Bilpakk/UI/Widgets/WBP_PauseAndEnd.WBP_PauseAndEnd_C|GetWBP_MapGrid (Variables|Default|GetPauseAndEndWidget)))) (delegate Custom|OnRowChanged))))))
    (:then_2
      ;[1 1 1] Bind events to action bar buttons
      (bind _aswbp_menu_action_bar (Utilities|Casting|CastToWBP_MenuActionBar (UserInterface|GetUserWidgetObject (Variables|Default|GetActionBar))))
      (bind _output_get (Variables|Default|SetActionBarWidget _aswbp_menu_action_bar))
      (Utilities|FlowControl|Sequence
        (:then_0
          (EventDispatchers|BindEventtoOnReleased (Variables|/Game/Bilpakk/UI/Widgets/WBP_MenuActionBar.WBP_MenuActionBar_C|GetNewGame _output_get) (delegate Custom|OnPressedPlay)))
        (:then_1
          (EventDispatchers|BindEventtoOnReleased (Variables|/Game/Bilpakk/UI/Widgets/WBP_MenuActionBar.WBP_MenuActionBar_C|GetContinue _output_get) (delegate Custom|ContinuePressed)))
        (:then_2
          (EventDispatchers|BindEventtoOnReleased (Variables|/Game/Bilpakk/UI/Widgets/WBP_MenuActionBar.WBP_MenuActionBar_C|GetMenu _output_get) (delegate Custom|MenuPressed)))
        (:then_3
          (EventDispatchers|BindEventtoOnReleased (Variables|/Game/Bilpakk/UI/Widgets/WBP_MenuActionBar.WBP_MenuActionBar_C|GetQuit _output_get) (delegate Custom|QuitPressed)))))
    (:then_3
      ;[1 1 1] End Game Widget
      (bind _aswbp_game_finished (Utilities|Casting|CastToWBP_GameFinished (UserInterface|GetUserWidgetObject (Variables|Default|GetPopOver))))
      (bind _output_get_2 (Variables|Default|SetEndGameWidget _aswbp_game_finished))
      (Widget|SetVisibility _output_get_2 "Collapsed")
      (Widget|SetIsEnabled _output_get_2 false)
      (EventDispatchers|BindEventtoOnReleased (Variables|/Game/Bilpakk/UI/Widgets/WBP_GameFinished.WBP_GameFinished_C|GetContinue _output_get_2) (delegate Custom|ContinueButtonClicked)))))

(event EventPause
  (bind _actionbarwidget (Variables|Default|GetActionBarWidget))
  ;[1 1 1] Pause
  (if (Variables|Default|GetIsFirst)
    (Variables|Default|SetIsFirst false)
    (Default|ShowLevelPicker (Variables|Default|GetPauseAndEndWidget))
    (else
      (Default|ShowHighscore (Variables|Default|GetPauseAndEndWidget))
      (Utilities|FlowControl|Sequence
        (:then_0
          (Default|EnableMenu _actionbarwidget))
        (:then_1
          (Default|EnableNewGame _actionbarwidget))
        (:then_2
          (Default|EnableContinue _actionbarwidget))))))

(event EventFinish
  (bind _endgamewidget (Variables|Default|GetEndGameWidget))
  (bind _actionbarwidget (Variables|Default|GetActionBarWidget))
  (bind _audio (Variables|Default|GetAudio))
  (bind _pauseandendwidget (Variables|Default|GetPauseAndEndWidget))
  (bind _points (Variables|/Game/Bilpakk/UI/Widgets/WBP_GameFinished.WBP_GameFinished_C|GetPoints _endgamewidget))
  (bind _font (Variables|/Script/UMG.TextBlock|GetFont _points))
  ;[1 1 1] Finish
  (Widget|SetVisibility _endgamewidget "Visible")
  (Widget|SetIsEnabled _endgamewidget true)
  (Audio|Components|Audio|SetSound _audio "/Game/Bilpakk/Sound/SFX/Drumroll.Drumroll")
  (Audio|Components|Audio|Play _audio 0.0)
  (Default|ShowHighscore _pauseandendwidget)
  (Widget|SetIsEnabled _pauseandendwidget false)
  (CallFunction|ResetUIRotation)
  (Widget|SetIsEnabled (Variables|Default|GetActionBarWidget) false)
  (Utilities|FlowControl|Sequence
    (:then_0
      (Default|EnableMenu _actionbarwidget))
    (:then_1
      (Default|EnableNewGame _actionbarwidget))
    (:then_2
      (Default|DisableContinue _actionbarwidget))
    (:then_3
      (bind (_direction _interpolation _textsize) (Timeline|AnimatePoints PlayFromStart)
        (:Update
          (Rendering|Components|TextRender|SetText _points (Utilities|Text|FormatText "{0} Poeng" (Math|Float|Floor (Math|Interpolation|Ease "EaseOut" _interpolation (Math|Float|MakeLiteralFloat 0.0) (Math|Conversions|ToFloat(Integer) (Class|BilpakkGameState|GetPoints)) 2.0))))
          (Class|TextBlock|SetFont _points (Utilities|Struct|MakeSlateFontInfo (.fontobject _font) (.fontmaterial _font) (.outlinesettings _font) (.typefacefontname _font) (Math|Float|Truncate _textsize) (.letterspacing _font))))))))

(fn ConstructionScript)

(fn ResetUIRotation)

(fn StartNewGame
  (bind _gamestate (Variables|Default|GetGameState))
  (bind _currentrow (Variables|Default|GetCurrentRow))
  (Utilities|IsValid _gamestate
    (:Is%20Valid
      (Class|BilpakkGameState|StartGame _gamestate _currentrow))
    (:Is%20Not%20Valid
      (Game|OpenLevel(byName) "Main" true (Utilities|String|ToString(Text) (Utilities|Text|FormatText "?RowName={0}" _currentrow))))))